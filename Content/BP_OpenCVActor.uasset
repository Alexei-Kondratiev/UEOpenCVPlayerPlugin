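; Actor that plays a video through an OpenCV player component onto a spinning billboard.
; BeginPlay resolves the file path, optionally under the project content directory, creates a dynamic M_OpenCV material, opens the stream, caches its properties, applies the frame range and starts playback.
; A next-frame callback pushes each decoded texture into the material's Texture parameter and records the frame index.
; Tick slowly rotates the actor on all three axes.
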(event `self.ReceiveBeginPlay`
  (bind _billboard (`self.Billboard`))
  (bind _opencvplayer (`self.OpenCVPlayer`))
  (bind _videofilename (`self.VideoFileName`))
  (`|ExecutionSequence`
    (:`then_0`
      (if (`self.UseContentDir`)
        (set `self.TmpVideoFileName` (`KismetStringLibrary.Concat_StrStr` (`OpenCVPlayerComponent.GetProjectContentDir` _opencvplayer) _videofilename))
        (else
          (set `self.TmpVideoFileName` _videofilename))))
    (:`then_1`
      (add `OpenCVPlayerComponent.OnNextVideoFrame` _opencvplayer (delegate `OnNextVideoFrame_Event_0`))
      (bind _returnvalue (`PrimitiveComponent.CreateDynamicMaterialInstance` _billboard 0 "/Game/M_OpenCV.M_OpenCV"))
      (`PrimitiveComponent.SetMaterial` _billboard 0 _returnvalue)
      (set `self.DynamicMaterial` _returnvalue)
      (bind _returnvalue_2 (`OpenCVPlayerComponent.OpenVideoStream` _opencvplayer (`self.TmpVideoFileName`)))
      (if _returnvalue_2
        (set `self.FrameCount` (`OpenCVPlayerComponent.GetFrameCount` _opencvplayer))
        (set `self.FrameRate` (`OpenCVPlayerComponent.GetFrameRate` _opencvplayer))
        (set `self.FrameSize` (`OpenCVPlayerComponent.GetFrameSize` _opencvplayer))
        (set `self.LoopPlayback` (`OpenCVPlayerComponent.GetLoopPlayback` _opencvplayer))
        (`OpenCVPlayerComponent.SetFrameStartIndex` _opencvplayer (`self.FrameStartIndex`))
        (`OpenCVPlayerComponent.SetFramesToPlay` _opencvplayer (`self.FramesToPlay`))
        (`OpenCVPlayerComponent.StartVideoStream` _opencvplayer)))))

(event `OnNextVideoFrame_Event_0`
  (bind _opencvplayer (`self.OpenCVPlayer`))
  (bind _returnvalue (`OpenCVPlayerComponent.GetFrameTexture` _opencvplayer))
  (`MaterialInstanceDynamic.SetTextureParameterValue` (`self.DynamicMaterial`) "Texture" _returnvalue)
  (set `self.NewFrameIndex` (`OpenCVPlayerComponent.GetNewFrameIndex` _opencvplayer)))

(event `self.ReceiveTick`
  (params (DeltaSeconds :type "Float (single-precision)"))
  (`self.K2_AddActorLocalRotation` (struct :`Pitch` 0.1 :`Yaw` 0.1 :`Roll` 0.1)))

(fn `UserConstructionScript`)